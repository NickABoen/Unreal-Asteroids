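; ShipState is a state Blueprint that stores the player's score and remaining lives for a ship game.
; Its functions add, reset and read PlayerScore, and set, take and read Lives.
; Score additions apply only for positive amounts, and taking lives clamps at zero, while setting lives assigns the value unchecked.
; It has no active event logic, so values change only through calls to these functions.
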(event EventBeginPlay)

(event EventTick
  (params (DeltaSeconds :type Float%20%28single-precision%29)))

(fn ConstructionScript)

(fn AddtoScore
  (params (Amount%20to%20Add :type Integer))
  (if (> Amount%20to%20Add 0)
    (Variables|Gameplay|SetPlayer%20Score (+ Amount%20to%20Add (Variables|Gameplay|GetPlayer%20Score)))))

(fn ResetScore
  (Variables|Gameplay|SetPlayer%20Score 0))

(fn GetScore
  (return (Variables|Gameplay|GetPlayer%20Score)))

(fn GetLives
  (return (Variables|Gameplay|GetLives)))

(fn TakeLife
  (params (Lives%20to%20Take :type Integer))
  (Variables|Gameplay|SetLives (Math|Integer|Max(Integer) (- (Variables|Gameplay|GetLives) Lives%20to%20Take))))

(fn SetLives
  (params (New%20Life%20Count :type Integer))
  (Variables|Gameplay|SetLives New%20Life%20Count))