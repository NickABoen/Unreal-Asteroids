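; Game state for an Asteroids clone that drives level progression and new-game resets.
; On a new level it waits briefly, resets score and lives if the level is negative, then increments the level.
; It has the spawner place large asteroids, their count scaling with level.
; The player easement box uses X/Z coordinates but has zero size, as its easement variable is unused.
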(event Custom|New%20Level
  (bind _returnvalue (Game|GetPlayerCharacter 0))
  (bind _level (Variables|Default|GetLevel))
  (bind _returnvalue_2 (Transformation|GetActorLocation _returnvalue))
  (bind (_x _y _z) (Math|Vector|BreakVector _returnvalue_2))
  (bind _returnvalue_3 (Math|Vector2D|MakeVector2D _x _z))
  (Utilities|FlowControl|Delay 1.0)
  (if (< _level 0)
    (CallFunction|ResetGame))
  (Math|Integer|IncrementInt _level ; Increment level
    (:%20%20
      (Default|SpawnAsteroidsAroundPlayer (Variables|Default|GetAsteroid%20Spawner) (+ (* _level (Variables|Default|GetAdditional%20Asteroids%20Per%20Level)) (Variables|Default|GetAsteroid%20Base%20Count)) "/Game/Blueprints/Asteroid_Large_BP.Asteroid_Large_BP_C" (Math|Box2D|MakeBox2D (- _returnvalue_3 0.0) (+ _returnvalue_3 0.0))))))

(fn ConstructionScript)

(fn ResetGame
  (bind _asship_state (Utilities|Casting|CastToShipState (Variables|/Script/Engine.Controller|GetPlayerState (Game|GetPlayerController 0))))
  (Default|ResetScore _asship_state)
  (bind _asasteroids_game_instance (Utilities|Casting|CastToAsteroids_Game_Instance (Game|GetGameInstance)))
  (Default|ResetScore _asasteroids_game_instance)
  (Default|SetLives _asship_state (Variables|Default|GetStarting%20Lives)))