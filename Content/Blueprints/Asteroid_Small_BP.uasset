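; Small asteroid actor for an Asteroids clone that starts a new level when it is the last asteroid left.
; On EndPlay it counts all AsteroidBase_BP actors and, if one or fewer exist, calls NewLevel on AsteroidsCloneGameState_BP.
; That call also requires a successful cast to Asteroids_Game_Instance, although its TriggerLevelChange call is left unconnected and never runs.
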(event EventBeginPlay
  (|CallParentFunction))

(event Collision|EventActorBeginOverlap
  (params (OtherActor :type Actor%20Object%20Reference))
  (|CallParentFunction OtherActor))

(event EventTick
  (params (DeltaSeconds :type Float%20%28single-precision%29)))

(event EventEndPlay
  (params (EndPlayReason :type EEndPlayReason%20Enum :default "Destroyed"))
  (bind _outactors (Actor|GetAllActorsOfClass "/Game/Blueprints/AsteroidBase_BP.AsteroidBase_BP_C"))
  (if (<= (Utilities|Array|Length _outactors) 1)
    (bind _asasteroids_game_instance (Utilities|Casting|CastToAsteroids_Game_Instance (Game|GetGameInstance)))
    (bind _asasteroids_clone_game_state_bp (Utilities|Casting|CastToAsteroidsCloneGameState_BP (Game|GetGameState)))
    (Default|NewLevel _asasteroids_clone_game_state_bp)))

(fn ConstructionScript
  (|CallParentFunction))