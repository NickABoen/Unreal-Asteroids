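; Component that keeps its owning actor inside the playing field by wrapping it to the opposite side, Asteroids-style.
; On BeginPlay it takes the PlayingField box from the first GameBounds actor and derives warp extents from its size plus padding, which AddExtentPadding can grow.
; Each Tick it teleports the owner using a per-axis, negative-safe vector modulo, treating the field as centered on the world origin.
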(event EventTick
  (params (DeltaSeconds :type Float%20%28single-precision%29))
  (bind _self self)
  (bind _warp_extents (Variables|Default|GetWarp%20Extents))
  (bind _returnvalue (Components|GetOwner _self))
  (Utilities|IsValid (Variables|Default|GetMovement%20Bounds)
    (:Is%20Valid
      (Transformation|SetActorLocation _returnvalue (- (Utilities|%(Vector) (+ (Transformation|GetActorLocation _returnvalue) _warp_extents) (* _warp_extents 2)) _warp_extents) false true))))

(event EventBeginPlay
  (bind _outactors (Actor|GetAllActorsOfClass "/Game/Blueprints/GameBounds.GameBounds_C"))
  (if (> (Utilities|Array|Length _outactors) 0)
    (Variables|Default|SetMovement%20Bounds (Variables|/Game/Blueprints/GameBounds.GameBounds_C|GetPlaying%20Field (Utilities|Array|Get(acopy) _outactors)))
    (CallFunction|RecomputeExtents)))

(fn AddExtentPadding
  (params (Additional%20ExtentsBox :type Vector))
  (Variables|Default|SetPadding%20Extents (+ Additional%20ExtentsBox (Variables|Default|GetPadding%20Extents)))
  (CallFunction|RecomputeExtents))

(fn RecomputeExtents
  (Variables|Default|SetWarp%20Extents (+ (Components|Box|GetScaledBoxExtent (Variables|Default|GetMovement%20Bounds)) (Variables|Default|GetPadding%20Extents))))