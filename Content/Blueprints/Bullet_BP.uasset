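; Player bullet actor for an asteroid-shooting game that destroys asteroids and awards points.
; On begin play it pads its BoundedPosition component by its bounds extent and launches along the arrow's forward vector at a fixed speed through ProjectileMovement.
; Overlapping an asteroid destroys both actors and adds the asteroid's score to the first player's ShipState.
; On end play, for any reason, it calls Give on its BulletCounter if valid.
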(event EventBeginPlay
  (bind _projectilemovement (Variables|Default|GetProjectileMovement))
  (Default|AddExtentPadding (Variables|Default|GetBoundedPosition) (Components|Box|GetScaledBoxExtent (Variables|Default|GetBounds)))
  (bind _output_get (Variables|/Script/Engine.ProjectileMovementComponent|SetInitialSpeed _projectilemovement (Variables|Movement|GetSpeed)))
  (bind _output_get_2 (Variables|/Script/Engine.ProjectileMovementComponent|SetMaxSpeed _projectilemovement _output_get))
  (Variables|/Script/Engine.MovementComponent|SetVelocity _projectilemovement (* (Math|Vector|GetForwardVector (Variables|Default|GetArrow)) _output_get_2)))

(event EventEndPlay
  (params (EndPlayReason :type EEndPlayReason%20Enum :default "Destroyed"))
  (bind _bullet_counter (Variables|Default|GetBullet%20Counter))
  (if (Utilities|IsValid _bullet_counter)
    (Default|Give _bullet_counter)))

(event Collision|EventActorBeginOverlap
  (params (OtherActor :type Actor%20Object%20Reference))
  (bind _asasteroid_base_bp (Utilities|Casting|CastToAsteroidBase_BP OtherActor))
  ;[1 1 1] Destroy Bullet
  (Actor|DestroyActor)
  ;[1 1 1] Update Score
  (bind _asship_state (Utilities|Casting|CastToShipState (Variables|/Script/Engine.Controller|GetPlayerState (Game|GetPlayerController 0)))
    (:then
      (Default|AddtoScore _asship_state (Default|GetScore _asasteroid_base_bp)))
    (:CastFailed
      _))
  (Actor|DestroyActor _asasteroid_base_bp))

(fn ConstructionScript)