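; Spawner actor that places asteroids at random points on the XZ plane, using an array of Box2D spawning zones.
; The construction script rebuilds a box component per zone.
; SpawnRandomAsteroids always spawns large asteroids at GetRandomSpawnLocation, which re-rolls the zone index for each bound, so zones can mix.
; SpawnAsteroidsAroundPlayer is unfinished, with no class or use of player bounds, and the exclusion-zone helpers are stubs.
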(fn ConstructionScript
  ;[1 1 1] Clear out current box components
  (for _array_element (Actor|GetComponentsByClass "/Script/Engine.BoxComponent")
    (Components|DestroyComponent _array_element))
  ;[1 1 1] Add box components for each box2d
  (for _array_element_2 (Variables|Default|GetSpawning%20Zones)
    (CallFunction|AddBoxCollisionfromBox2D _array_element_2)))

(fn AddBoxCollisionfromBox2D
  (params (Box2D :type Box%202D%20Structure))
  (bind (_min _max) (Utilities|Struct|BreakBox2D Box2D))
  (bind _min_2 (Utilities|Struct|BreakBox2D Box2D))
  (bind (_x _y) (Math|Vector2D|BreakVector2D _min))
  (bind (_x_2 _y_2) (Math|Vector2D|BreakVector2D _max))
  (bind (_x_3 _y_3) (Math|Vector2D|BreakVector2D _min_2))
  (LocalVariables|SetBox%20Extents (Math|Vector|MakeVector (/ (- _x_2 _x) 2.0) 0.0 (/ (- _y_2 _y) 2.0)))
  (LocalVariables|SetBox%20Location (Math|Vector|MakeVector (+ _x_3 (.X (Math|Vector|BreakVector (LocalVariables|GetBox%20Extents)))) 0.0 (+ _y_3 (.Z (Math|Vector|BreakVector (LocalVariables|GetBox%20Extents))))))
  (bind _returnvalue (AddComponent|AddBoxComponent false (Math|Conversions|ToTransform(Vector) (LocalVariables|GetBox%20Location))))
  (Components|Box|SetBoxExtent _returnvalue (LocalVariables|GetBox%20Extents) true))

(fn SpawnRandomAsteroids
  (params (Number%20to%20Spawn :type Integer) (Type%20to%20spawn :type Asteroid%20Base%20BP%20Class%20Reference))
  (for _index (range 0 (- Number%20to%20Spawn 1))
    (bind _location (CallFunction|GetRandomSpawnLocation))
    (Game|SpawnActorfromClass "/Game/Blueprints/Asteroid_Large_BP.Asteroid_Large_BP_C" (Math|Conversions|ToTransform(Vector) _location) "Undefined" 0 0)))

(fn GetRandomSpawnLocation
  (bind _spawning_zones (Variables|Default|GetSpawning%20Zones))
  (bind _returnvalue (Utilities|Array|Length _spawning_zones))
  (bind _returnvalue_2 (Math|Random|RandomInteger _returnvalue))
  (bind _item (Utilities|Array|Get(acopy) _spawning_zones _returnvalue_2))
  (bind (_min _max) (Utilities|Struct|BreakBox2D _item))
  (bind (_x _y) (Math|Vector2D|BreakVector2D _min))
  (bind (_x_2 _y_2) (Math|Vector2D|BreakVector2D _max))
  (return (Math|Vector|MakeVector (Math|Random|RandomFloatinRange _x _x_2) 0.0 (Math|Random|RandomFloatinRange _y _y_2))))

(fn SpawnAsteroidsAroundPlayer
  (params (Number%20to%20Spawn :type Integer) (Type%20to%20Spawn :type Asteroid%20Base%20BP%20Class%20Reference) (Player%20Easement%20Bounds :type Box%202D%20Structure))
  (for _index (range 0 (- Number%20to%20Spawn 1))
    (bind _location (CallFunction|GetRandomSpawnLocation))
    (Game|SpawnActorfromClass 0 (Math|Conversions|ToTransform(Vector) _location) "Undefined" 0 0)))