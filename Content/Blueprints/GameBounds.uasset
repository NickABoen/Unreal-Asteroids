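; GameBounds is an actor defining a box playing field on the X-Z plane, enclosed by four barrier boxes.
; Its construction script sizes the field from FieldExtents and Depth, sets the actor's Y to Depth, then fits Left, Right, Top and Bottom barriers outside its edges using BarrierWidth.
; MoveActorToFieldEdge teleports actors listed in OffscreenActors to a given direction times twice the field extent, in world space.
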(fn ConstructionScript
  (CallFunction|UpdatePlayingField)
  (CallFunction|UpdateBarriers))

(fn UpdatePlayingField
  (bind _fieldextents (Variables|Bounds|GetFieldExtents))
  (bind _depth (Variables|Bounds|GetDepth))
  (bind (_x _y) (Math|Vector2D|BreakVector2D _fieldextents))
  (Components|Box|SetBoxExtent (Variables|Default|GetPlaying%20Field) (Math|Vector|MakeVector _x _depth _y) true)
  (Transformation|SetActorLocation (+ (Math|Vector|MakeVector 0.0 _depth 0.0) (* (Transformation|GetWorldLocation (Variables|Default|GetPlaying%20Field)) "1.000000, 0,1.000000")) false false))

(fn UpdateBarriers
  (bind _left (Variables|Default|GetLeft))
  (bind _right (Variables|Default|GetRight))
  (bind _top (Variables|Default|GetTop))
  (bind _bottom (Variables|Default|GetBottom))
  (Utilities|FlowControl|Sequence
    (:then_0
      ;[1 1 1] Set barrier size relative to playing field
      (Components|Box|SetBoxExtent (Variables|Default|GetLeft) (+ (* (Components|Box|GetUnscaledBoxExtent (Variables|Default|GetPlaying%20Field)) "0,1.000000,1.000000") (* "1.000000, 0, 0" (Variables|Bounds|GetBarrierWidth))) true))
    (:then_1
      (Components|Box|SetBoxExtent (Variables|Default|GetRight) (+ (* (Components|Box|GetUnscaledBoxExtent (Variables|Default|GetPlaying%20Field)) "0,1.000000,1.000000") (* "1.000000, 0, 0" (Variables|Bounds|GetBarrierWidth))) true))
    (:then_2
      (Components|Box|SetBoxExtent (Variables|Default|GetTop) (+ (* (Components|Box|GetUnscaledBoxExtent (Variables|Default|GetPlaying%20Field)) "1.000000,1.000000,0.000000") (* "0.000000, 0,1.000000" (Variables|Bounds|GetBarrierWidth))) true))
    (:then_3
      (Components|Box|SetBoxExtent (Variables|Default|GetBottom) (+ (* (Components|Box|GetUnscaledBoxExtent (Variables|Default|GetPlaying%20Field)) "1.000000,1.000000,0.000000") (* "0.000000, 0,1.000000" (Variables|Bounds|GetBarrierWidth))) true))
    (:then_4
      (Utilities|FlowControl|Sequence
        (:then_0
          ;[1 1 1] Set barreir position relative to playing field
          (Transformation|SetRelativeLocation _left (* (+ (Components|Box|GetUnscaledBoxExtent _left) (Components|Box|GetUnscaledBoxExtent (Variables|Default|GetPlaying%20Field))) "-1.000000, 0, 0") false false))
        (:then_1
          (Transformation|SetRelativeLocation _right (* (+ (Components|Box|GetUnscaledBoxExtent _right) (Components|Box|GetUnscaledBoxExtent (Variables|Default|GetPlaying%20Field))) "1.000000, 0, 0") false false))
        (:then_2
          (Transformation|SetRelativeLocation _top (* (+ (Components|Box|GetUnscaledBoxExtent _top) (Components|Box|GetUnscaledBoxExtent (Variables|Default|GetPlaying%20Field))) "0.000000, 0,1.000000") false false))
        (:then_3
          (Transformation|SetRelativeLocation _bottom (* (+ (Components|Box|GetUnscaledBoxExtent _bottom) (Components|Box|GetUnscaledBoxExtent (Variables|Default|GetPlaying%20Field))) "0.000000, 0,-1.000000") false false))))))

(fn MoveActortoFieldEdge
  (params (Actor :type Actor%20Object%20Reference) (Unit%20Vector%20Direction :type Vector))
  (if (Utilities|Set|Contains (Variables|Default|GetOffscreenActors) Actor)
    (Transformation|SetActorLocation Actor (* Unit%20Vector%20Direction (* (Components|Box|GetScaledBoxExtent (Variables|Default|GetPlaying%20Field)) 2)) false true)))