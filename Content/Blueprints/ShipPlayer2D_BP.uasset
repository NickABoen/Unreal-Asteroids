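; Player ship Character for a 2D Asteroids game, with thrust, rotation, limited shooting and lives.
; Thrust adds force along the capsule's up vector, capped by max speed and slowed through physics volume fluid friction, while the Thruster animation loops between set frames.
; BulletTracker gates firing.
; Asteroid hits spend a ShipState life to respawn at origin with flashing invulnerability, or save score to the GameInstance and open Game_Over.
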(event EventTick
  (params (DeltaSeconds :type Float%20%28single-precision%29))
  (CallFunction|AnimationTick 0.0)
  (CallFunction|ShipThrusting)
  (CallFunction|KeepFluidFrictionUptoDate)
  (CallFunction|MaintainMaxSpeed)
  (if (Variables|Gameplay|GetisInvulnerable)
    (Utilities|FlowControl|Delay (Variables|Gameplay|GetSpawn%20Invulnerability%20Time))
    (Variables|Gameplay|SetisInvulnerable false)))

(event EventBeginPlay
  (CallFunction|InitializeFluidFriction)
  (CallFunction|InitializeMaxFlyingSpeed)
  (Default|AddExtentPadding (Variables|Default|GetBoundedPosition) (Components|Box|GetScaledBoxExtent (Variables|Default|GetBoundingBox)))
  (Audio|Components|Audio|Stop (Variables|Default|GetThruster)))

(event EventStartThrust
  (Variables|Movement|SetIsThrusting true)
  (CallFunction|BeginThrustAnim))

(event EventEndThrust
  (Variables|Movement|SetIsThrusting false)
  (CallFunction|EndThrustAnim))

(event EventTurnLeft
  (params (AxisValue :type Float%20%28single-precision%29))
  (CallFunction|ShipRotation AxisValue))

(event EventTurnRight
  (params (AxisValue :type Float%20%28single-precision%29))
  (CallFunction|ShipRotation AxisValue))

(event Input|ActionEvents|InputActionFire
  (params (Key :type Key%20Structure :default "AnyKey"))
  (:Pressed
    (bind _is_valid (Default|TrytoTake (Variables|Default|GetBullet%20Tracker)))
    (if _is_valid
      (CallFunction|ShootBullet))))

(event Collision|EventActorBeginOverlap
  (params (OtherActor :type Actor%20Object%20Reference))
  (if (not (Variables|Gameplay|GetisInvulnerable))
    (bind _asasteroid_base_bp (Utilities|Casting|CastToAsteroidBase_BP OtherActor))
    (CallFunction|KillPlayer)
    (Actor|DestroyActor _asasteroid_base_bp)))

(event Custom|Respawn
  ;[1 1 1] Make player invulnerable
  (CallFunction|StartInvulnerability)
  ;[1 1 1] Remove a life from the player
  (bind _asship_state (Utilities|Casting|CastToShipState (Variables|/Script/Engine.Controller|GetPlayerState (Game|GetPlayerController 0))))
  (Default|TakeLife _asship_state 1)
  ;[1 1 1] Kill the players current velocity and teleport them to the center
  (Variables|/Script/Engine.MovementComponent|SetVelocity (Variables|Character|GetCharacterMovement) "0, 0, 0")
  (Transformation|SetActorTransform self (Math|Transform|MakeTransform "0, 0, 0" "0,0.000000, 0") false true))

(event Custom|Kill%20Player
  ;[1 1 1] Check Player Lives
  (bind _asship_state (Utilities|Casting|CastToShipState (Variables|/Script/Engine.Controller|GetPlayerState (Pawn|GetController))))
  (if (> (Default|GetLives _asship_state) 0)
    ;[1 1 1] Respawn Ship
    (CallFunction|Respawn)
    (else
      ;[1 1 1] End Game
      (bind _asasteroids_game_instance (Utilities|Casting|CastToAsteroids_Game_Instance (Game|GetGameInstance)))
      (bind _asship_state_2 (Utilities|Casting|CastToShipState (Variables|Default|GetPlayerState)))
      (bind _player_score (Default|GetScore _asship_state_2))
      (Default|SetScore _asasteroids_game_instance (Math|Conversions|ToFloat(Integer) _player_score))
      (Game|OpenLevel(byName) "Game_Over" false))))

(event Custom|Start%20Invulnerability
  (Variables|Gameplay|SetisInvulnerable true)
  (CallFunction|Flash)
  (Utilities|FlowControl|Delay (Variables|Gameplay|GetSpawn%20Invulnerability%20Time))
  (CallFunction|EndInvulnerability))

(event Custom|End%20Invulnerability
  (Variables|Gameplay|SetisInvulnerable false)
  (Rendering|SetActorHiddenInGame true))

(event Custom|Flash
  (if (Variables|Gameplay|GetisInvulnerable)
    (Utilities|FlowControl|Delay (Variables|Gameplay|GetInvulnerability%20Flash%20Span))
    (Rendering|SetActorHiddenInGame (not (Variables|Default|GetbHidden)))
    (CallFunction|Flash)))

(event Custom|Animation%20Tick
  (params (Delta%20Seconds :type Float%20%28single-precision%29))
  (bind _thruster (Variables|Default|GetThruster))
  (bind _thruster_2 (Variables|Default|GetThruster))
  (bind _returnvalue (Class|PaperFlipbookComponent|GetPlaybackPositioninFrames _thruster))
  (if (and (Variables|Movement|GetIsThrusting) (== (Variables|Animation|GetEnd%20Cycle%20Frame) _returnvalue)) ; End of Cycle
    (Class|PaperFlipbookComponent|SetPlaybackPositioninFrames _thruster_2 (Variables|Animation|GetStart%20Cycle%20Frame) true)
    (elif (== _returnvalue (Variables|Animation|GetEnd%20Thrust%20Frame)) ; End of animation
      (Audio|Components|Audio|Stop _thruster_2))))

(event Custom|Begin%20Thrust%20Anim
  (Components|Timeline|PlayfromStart (Variables|Default|GetThruster)))

(event Custom|End%20Thrust%20Anim
  (Class|PaperFlipbookComponent|SetPlaybackPositioninFrames (Variables|Default|GetThruster) (Variables|Animation|GetEnd%20Cycle%20Frame) false))

(fn ConstructionScript
  (Audio|Components|Audio|Stop (Variables|Default|GetThruster)))

(fn ShipThrusting
  (bind _charactermovement (Variables|Character|GetCharacterMovement))
  (if (Variables|Movement|GetIsThrusting)
    (Physics|AddForce _charactermovement (* (Math|Vector|GetUpVector (Variables|Default|GetCapsuleComponent)) (* (Variables|Movement|GetAcceleration) (Variables|/Script/Engine.CharacterMovementComponent|GetMass _charactermovement))))))

(fn ShipRotation
  (params (Rotation%20Multiplier :type Float%20%28single-precision%29))
  (Pawn|Input|AddControllerPitchInput (* Rotation%20Multiplier (Variables|Movement|GetRotationRate))))

(fn KeepFluidFrictionUptoDate
  (bind _braking (Variables|Movement|GetBraking))
  (bind _charactermovement (Variables|Character|GetCharacterMovement))
  (bind _returnvalue (Class|MovementComponent|GetPhysicsVolume _charactermovement))
  (if (!= _braking (Variables|/Script/Engine.PhysicsVolume|GetFluidFriction _returnvalue))
    (Variables|/Script/Engine.PhysicsVolume|SetFluidFriction _returnvalue _braking)))

(fn MaintainMaxSpeed
  (bind _charactermovement (Variables|Character|GetCharacterMovement))
  (Variables|/Script/Engine.MovementComponent|SetVelocity _charactermovement (Math|Vector|ClampVectorSize (Variables|/Script/Engine.MovementComponent|GetVelocity _charactermovement) 0.0 (Variables|/Script/Engine.CharacterMovementComponent|GetMaxFlySpeed _charactermovement))))

(fn InitializeFluidFriction
  (Variables|/Script/Engine.PhysicsVolume|SetFluidFriction (Class|MovementComponent|GetPhysicsVolume (Variables|Character|GetCharacterMovement)) (Variables|Movement|GetBraking)))

(fn InitializeMaxFlyingSpeed
  (Variables|/Script/Engine.CharacterMovementComponent|SetMaxFlySpeed (Variables|Character|GetCharacterMovement) (Variables|Movement|GetMax%20Speed)))

(fn ShootBullet
  (bind _self self)
  (Game|SpawnActorfromClass "/Game/Blueprints/Bullet_BP.Bullet_BP_C" (Math|Transform|MakeTransform (Transformation|GetWorldLocation (Variables|Default|GetGunpoint)) (Transformation|GetActorRotation _self) "4.000000,1.000000,4.000000") "Undefined" _self (Variables|Default|GetBullet%20Tracker) (Game|GetInstigator _self)))