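; Base 2D asteroid actor that drifts and spins, can break into spawned pieces, and exposes a score value.
; BeginPlay picks a random sprite, X-Z velocity and pitch spin for the movement components, then pads BoundedPosition by the asteroid's extent.
; Destroyed calls BreakAsteroid, which destroys the actor and, if CanBreak, spawns BreakCount actors of BreakSpawnClass at its transform.
; Overlap casts to bullet and player ship but takes no action.
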(event EventBeginPlay
  (Utilities|FlowControl|Sequence
    (:then_0
      (CallFunction|AssignRandomVelocity))
    (:then_1
      (CallFunction|AssignRandomRotationRate))
    (:then_2
      (bind _result (CallFunction|GetRandomSprite))
      (Rendering|Components|Sprite|SetSprite (Variables|Default|GetRenderComponent) _result))
    (:then_3
      (Default|AddExtentPadding (Variables|Default|GetBoundedPosition) (Components|Box|GetScaledBoxExtent (Variables|Default|GetBounds))))))

(event EventDestroyed
  (CallFunction|BreakAsteroid))

(event Collision|EventActorBeginOverlap
  (params (OtherActor :type Actor%20Object%20Reference))
  (Utilities|Casting|CastToBullet_BP OtherActor
    (:CastFailed
      (Utilities|Casting|CastToShipPlayer2D_BP OtherActor))))

(fn ConstructionScript)

(fn GetRandomSprite
  (bind _sprite_set (Variables|Appearance|GetSprite%20Set))
  (return (Utilities|Array|Get(acopy) _sprite_set (Math|Random|RandomInteger (Utilities|Array|Length _sprite_set)))))

(fn BreakAsteroid
  (bind _self self)
  (Actor|DestroyActor)
  (if (Variables|Asteroid|GetCan%20Break)
    (for _index (range 1 (Variables|Asteroid|GetBreak%20Count))
      (Game|SpawnActorfromClass (Variables|Asteroid|GetBreak%20Spawn%20Class) (Transformation|GetActorTransform _self) (Variables|Default|GetSpawnCollisionHandlingMethod _self) _self (Game|GetInstigator _self)))))

(fn GetRandomVelocity
  (return (* (Math|Vector|Normalize (Math|Vector|MakeVector (Math|Random|RandomFloatinRange -1.0 1.0) 0.0 (Math|Random|RandomFloatinRange -1.0 1.0))) (Math|Random|RandomFloatinRange (Variables|Movement|GetMin%20Speed) (Variables|Movement|GetMax%20Speed)))))

(fn GetRandomRotation
  (return (Math|Rotator|MakeRotator 0.0 (Math|Random|RandomFloatinRange (Variables|Movement|GetMin%20Rotation%20Rate) (Variables|Movement|GetMax%20Rotation%20Rate)) 0.0)))

(fn AssignRandomVelocity
  (bind _return_value (CallFunction|GetRandomVelocity))
  (Variables|/Script/Engine.MovementComponent|SetVelocity (Variables|Default|GetProjectileMovement) _return_value))

(fn AssignRandomRotationRate
  (bind _return_value (CallFunction|GetRandomRotation))
  (Variables|/Script/Engine.RotatingMovementComponent|SetRotationRate (Variables|Default|GetRotatingMovement) _return_value))

(fn GetScore
  (return (Variables|Default|GetScore)))