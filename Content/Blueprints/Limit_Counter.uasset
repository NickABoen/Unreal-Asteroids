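; Limit counter Blueprint that tracks a count of available uses, starting at MaxCount on BeginPlay.
; TryToTake decrements the count while it is above zero, but returns false on both branches, so callers cannot tell whether a take succeeded.
; Give increments the count and applies modulo MaxCount, so it wraps around instead of clamping at the limit.
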(event EventBeginPlay
  (Variables|Default|SetCurrent%20Value (Variables|Default|GetMax%20Count)))

(event EventTick
  (params (DeltaSeconds :type Float%20%28single-precision%29)))

(fn TrytoTake
  (if (> (Variables|Default|GetCurrent%20Value) 0)
    (Math|Integer|DecrementInt (Variables|Default|GetCurrent%20Value)
      (:%20%20
        (return false)))
    (else
      (return false))))

(fn Give
  (bind _result (Math|Integer|IncrementInt (Variables|Default|GetCurrent%20Value))
    (:%20%20
      (Variables|Default|SetCurrent%20Value (Math|Integer|%(Integer) _result (Variables|Default|GetMax%20Count))))))