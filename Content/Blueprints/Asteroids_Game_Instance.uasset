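; Game Instance for an Asteroids game that holds score, current level and recent player lives across level loads.
; Simple getter, add, reset and set functions expose the recent score, and getter, add and reset functions manage the level counter.
; Player lives are only readable here through a getter; no function in this asset changes them.
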(fn GetScore
  (return (Variables|Default|GetRecent%20Score)))

(fn AddScore
  (params (Amount :type Float%20%28single-precision%29))
  (Variables|Default|SetRecent%20Score (+ Amount (Variables|Default|GetRecent%20Score))))

(fn ResetScore
  (Variables|Default|SetRecent%20Score 0.0))

(fn GetLevel
  (return (Variables|Default|GetCurrent%20Level)))

(fn AddLevel
  (params (Levels%20To%20Add :type Integer))
  (Variables|Default|SetCurrent%20Level (+ Levels%20To%20Add (Variables|Default|GetCurrent%20Level))))

(fn ResetLevel
  (Variables|Default|SetCurrent%20Level 0))

(fn GetRecentPlayerLives
  (return (Variables|Default|GetRecent%20Player%20Lives)))

(fn SetScore
  (params (New%20Score :type Float%20%28single-precision%29))
  (Variables|Default|SetRecent%20Score New%20Score))